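; BP_SkillBase is the base skill Blueprint for InvokerWars, providing the check for whether a skill can be cast.
; CanBeCasted returns true when the skill is off cooldown and the supplied available mana covers its cost.
; It gets both values through CheckManaCost, which reads SkillData.ManaCost, and CheckInCooldown, which returns the InCooldown flag.
; The event graph and construction script are empty, so this file neither spends mana nor updates the cooldown.
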(fn `CanBeCasted`
  (params (ManaAvailable :type "Float (double-precision)"))
  (returns (CanBeCasted :type Boolean))
  (bind _cost (`self.CheckManaCost`))
  (bind _incooldown (`self.CheckInCooldown`))
  (return (and (not _incooldown) (>= ManaAvailable _cost))))

(fn `CheckInCooldown`
  (returns (InCooldown :type Boolean))
  (return (`self.inCooldown`)))

(fn `CheckManaCost`
  (returns (Cost :type "Float (double-precision)"))
  (return (`.ManaCost_11_A20F5A1D4A4F81DC8B1B4F8715C96E8F` (break `/Game/InvokerWars/Blueprints/Skills/Base/STRUCT_SkillData` (`self.SkillData`)))))

(fn `UserConstructionScript`)