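; Base projectile for InvokerWars that homes in on a target actor and damages it on contact.
; On BeginPlay it sets the ProjectileMovement homing target to a scene component found on TargetActor.
; Overlaps with that target apply a fixed amount of damage and print the result, while other actors are ignored.
; The projectile does not destroy itself on hit in this graph.
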(event `self.ReceiveBeginPlay`
  (set `ProjectileMovementComponent.HomingTargetComponent` (`self.GetComponentByClass` (`self.TargetActor`) "/Script/Engine.SceneComponent") (`self.ProjectileMovement`)))

(event `self.ReceiveActorBeginOverlap`
  (params (OtherActor :type "Actor Object Reference"))
  (bind _targetactor (`self.TargetActor`))
  (if (== OtherActor _targetactor)
    (bind _returnvalue (`GameplayStatics.ApplyDamage` _targetactor 15.0))
    (`KismetSystemLibrary.PrintString` (`KismetStringLibrary.Conv_DoubleToString` _returnvalue))))

(fn `UserConstructionScript`)