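; HeroPlayerController is a player controller that handles mouse-driven unit selection.
; On BeginPlay it sets Game and UI input with the cursor always locked to the viewport and visible during capture.
; Left mouse press and release send start and stop selection messages to the HUD.
; Add and remove functions maintain a duplicate-free SelectedUnits array and notify each valid unit through OnUnitSelected.
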(event `self.ReceiveBeginPlay`
  (`WidgetBlueprintLibrary.SetInputMode_GameAndUIEx` self null "LockAlways" false))

(event `Key|LeftMouseButton`
  (params (Key :type "Key Structure"))
  (bind _returnvalue (`self.GetHUD`))
  (:`Pressed`
    (message `/Game/InvokerWars/Blueprints/UI/IHUDSelection.StartSelection` _returnvalue))
  (:`Released`
    (message `/Game/InvokerWars/Blueprints/UI/IHUDSelection.StopSelection` _returnvalue)))

(fn `AddToUnitSelection`
  (params (UnitToAdd :type "/Game/InvokerWars/Blueprints/Characters/Base/UnitBase Object Reference"))
  (`/Engine/EditorBlueprintResources/StandardMacros.IsValid` UnitToAdd
    (:`Is Valid`
      (`KismetArrayLibrary.Array_AddUnique` (`self.SelectedUnits`) UnitToAdd)
      (`/Game/InvokerWars/Blueprints/Characters/Base/UnitBase.OnUnitSelected` UnitToAdd true))))

(fn `RemoveFromUnitSelection`
  (params (UnitToRemove :type "/Game/InvokerWars/Blueprints/Characters/Base/UnitBase Object Reference"))
  (`/Engine/EditorBlueprintResources/StandardMacros.IsValid` UnitToRemove
    (:`Is Valid`
      (`KismetArrayLibrary.Array_RemoveItem` (`self.SelectedUnits`) UnitToRemove)
      (`/Game/InvokerWars/Blueprints/Characters/Base/UnitBase.OnUnitSelected` UnitToRemove false))))

(fn `UserConstructionScript`)