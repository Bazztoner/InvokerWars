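; Player camera actor that becomes player 0's view target on BeginPlay and provides mouse edge-scroll panning.
; Each Tick, horizontal and vertical functions compare the cursor's viewport position, as a fraction of viewport size, against ClosenessFactor margins.
; Near an edge they set DirectionVector from CameraSpeed, then add it to the root's relative location along Y or X, without delta-time scaling.
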(event `self.ReceiveBeginPlay`
  (`PlayerController.SetViewTargetWithBlend` (`GameplayStatics.GetPlayerController` 0) self 0.0 "VTBlend_Linear" 0.0 false))

(event `self.ReceiveTick`
  (params (DeltaSeconds :type "Float (single-precision)"))
  (`self.HorizontalMovement`)
  (`self.VerticalMovement`))

(fn `HorizontalMovement`
  (locals (DirectionVector :type "Vector Structure"))
  (bind _returnvalue_x (`KismetMathLibrary.BreakVector2D` (`WidgetLayoutLibrary.GetViewportSize`)))
  (bind _closenessfactor (`self.ClosenessFactor`))
  (bind _cameraspeed (`self.CameraSpeed`))
  (bind _returnvalue (`WidgetLayoutLibrary.GetMousePositionOnViewport`))
  (`|ExecutionSequence`
    (:`then_0`
      (bind _returnvalue_2 (/ (`KismetMathLibrary.BreakVector2D` _returnvalue) _returnvalue_x))
      (if (>= _returnvalue_2 (- 1.0 _closenessfactor))
        (set `local.DirectionVector` (`KismetMathLibrary.MakeVector` 0.0 _cameraspeed))
        (elif (<= _returnvalue_2 _closenessfactor)
          (set `local.DirectionVector` (`KismetMathLibrary.MakeVector` 0.0 (* _cameraspeed -1.0))))))
    (:`then_1`
      (`SceneComponent.K2_AddRelativeLocation` (`self.DefaultSceneRoot`) (`local.DirectionVector`) false false))))

(fn `UserConstructionScript`)

(fn `VerticalMovement`
  (locals (DirectionVector :type "Vector Structure"))
  (bind (_returnvalue_x _returnvalue_y) (`KismetMathLibrary.BreakVector2D` (`WidgetLayoutLibrary.GetViewportSize`)))
  (bind _closenessfactor (`self.ClosenessFactor`))
  (bind _cameraspeed (`self.CameraSpeed`))
  (bind _returnvalue (`WidgetLayoutLibrary.GetMousePositionOnViewport`))
  (`|ExecutionSequence`
    (:`then_0`
      (bind _returnvalue_2 (/ (`.Y` (`KismetMathLibrary.BreakVector2D` _returnvalue)) _returnvalue_y))
      (if (>= _returnvalue_2 (- 1.0 _closenessfactor))
        (set `local.DirectionVector` (`KismetMathLibrary.MakeVector` (* _cameraspeed -1.0)))
        (elif (<= _returnvalue_2 _closenessfactor)
          (set `local.DirectionVector` (`KismetMathLibrary.MakeVector` _cameraspeed)))))
    (:`then_1`
      (`SceneComponent.K2_AddRelativeLocation` (`self.DefaultSceneRoot`) (`local.DirectionVector`) false false))))